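; BP_Spring is a Paper2D spring pad that bounces any Character overlapping it, so enemies can use it as well as the player.
; The CharacterCheck overlap launches the Character along the spring's up vector scaled by BouncePower, overriding its vertical velocity.
; The flipbook then plays the active animation once without looping, and its finished-playing event swaps back to the idle flipbook.
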(event OnComponentBeginOverlap(CharacterCheck)
  (params (OverlappedComponent :type Primitive%20Component%20Object%20Reference) (OtherActor :type Actor%20Object%20Reference) (OtherComp :type Primitive%20Component%20Object%20Reference) (OtherBodyIndex :type Integer) (bFromSweep :type Boolean) (SweepResult :type Hit%20Result%20Structure%20%28by%20ref%29))
  ;[1 0.2552 0.2552] Is for the main class, so enemies also can use it
  (bind _ascharacter (Utilities|Casting|CastToCharacter OtherActor))
  ;[1 0.9202 0.2854] Launch action
  (Character|LaunchCharacter _ascharacter (* (Math|Vector|VectorUp) (Variables|Default|GetBouncePower)) false true)
  ;[1 0.83 0.1649] Stop the loop, so only do once
  (Components|Timeline|SetLooping (Variables|Default|GetPaperFlipbook) false)
  ;[0.08646 1 0.001098] Active the spring flipbook
  (Sprite|SetFlipbook (Variables|Default|GetPaperFlipbook) "/Game/PaperAssets/Spring/Spring__Active.Spring__Active")
  ;[1 0.224 0.224] Restarts the animation afterwards
  (Audio|Components|Audio|Play (Variables|Default|GetPaperFlipbook)))

(event OnFinishedPlaying(PaperFlipbook)
  ;[1 1 1] This will trigger after finish every execution
  (Sprite|SetFlipbook (Variables|Default|GetPaperFlipbook) "/Game/PaperAssets/Spring/Spring__Idle_PNG1_Flipbook.Spring__Idle_PNG1_Flipbook"))

(event EventBeginPlay)

(event Collision|EventActorBeginOverlap
  (params (OtherActor :type Actor%20Object%20Reference)))

(event EventTick
  (params (DeltaSeconds :type Float%20%28single-precision%29)))

(fn ConstructionScript)