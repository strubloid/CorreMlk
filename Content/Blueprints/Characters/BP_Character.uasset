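; Base 2D sprite character Blueprint that provides defeat handling.
; Defeat runs once via the IsDefeated flag, disabling capsule collision and the movement plane constraint, then launching the character along world up and right axes using tunable strengths.
; It forces the animation to the defeat state through a JumpDefeated jump node and raises the sprite's translucent sort priority so the body draws in front.
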(event Custom|Defeat
  ;[0.5837 1 0.5757] When this is triggered we need to check if isnt defeated, so only in this case we can set the defeated to true
  (if (not (Variables|Default|GetIsDefeated))
    (Variables|Default|SetIsDefeated true)
    ;[1 0.2691 0.2691] We remove the colision afterwards
    (Collision|SetCollisionEnabled (Variables|Default|GetCapsuleComponent) "NoCollision")
    ;[1 1 1] As we have on Character moviment constrain to plane, we will need to turn off before launch the character
    (Class|MovementComponent|SetPlaneConstraintEnabled (Variables|Character|GetCharacterMovement) false)
    (CallFunction|LaunchonDefeat)
    ;[0.4231 0.6807 1] This is triggering the Jump, so we dont need to implement death for all cases
    (Class|PaperZDAnimInstance|JumptoNode (Class|PaperZDCharacter|GetAnimInstance) "JumpDefeated" "None")
    ;[1 0.9458 0.1892] This is a way to make sure when you are dead, you will be shown in the front of it
    (Rendering|SetTranslucentSortPriority (Variables|Default|GetSprite) 1000)))

(event EventBeginPlay)

(event Collision|EventActorBeginOverlap
  (params (OtherActor :type Actor%20Object%20Reference)))

(event EventTick
  (params (DeltaSeconds :type Float%20%28single-precision%29)))

(fn ConstructionScript)

(fn LaunchonDefeat
  (Character|LaunchCharacter (+ (* (Math|Vector|GetUpVector "0, 0, 0") (Variables|Default|GetDefeatUpLaunch)) (* (Math|Vector|GetRightVector "0, 0, 0") (Variables|Default|GetDefeatForwardLaunch))) true true))