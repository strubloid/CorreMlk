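; Base or standalone enemy character (Pig folder) that turns around at walls and ledges.
; Each tick, while on a walkable floor, it checks whether the LedgeDetector overlaps any actor and flips 180 degrees if none is found.
; An overlap beginning on the Walldetector component triggers the same RotateCharacter flip.
; The floor check prevents repeated flipping while airborne.
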(event OnComponentBeginOverlap(Walldetector)
  (params (OverlappedComponent :type Primitive%20Component%20Object%20Reference) (OtherActor :type Actor%20Object%20Reference) (OtherComp :type Primitive%20Component%20Object%20Reference) (OtherBodyIndex :type Integer) (bFromSweep :type Boolean) (SweepResult :type Hit%20Result%20Structure%20%28by%20ref%29))
  (CallFunction|RotateCharacter))

(event EventBeginPlay)

(event Collision|EventActorBeginOverlap
  (params (OtherActor :type Actor%20Object%20Reference)))

(event EventTick
  (params (DeltaSeconds :type Float%20%28single-precision%29))
  (|CallParentFunction DeltaSeconds)
  ;[1 1 1] Detection of something, in this case will be the ledge
  (CallFunction|CheckLedge))

(fn ConstructionScript
  (|CallParentFunction))

(fn RotateCharacter
  ;[1 0.3262 0.2274] This is the way to rotate the enemy character
  (Transformation|SetActorRotation (Math|Rotator|CombineRotators (Transformation|GetActorRotation) "0.000000,180.000000,0.000000")))

(fn CheckLedge
  ;[0.5953 0.9367 1] Checking if the character is on the floor, otherwise it can be rotating auround the air
  (if (.bwalkablefloor (Variables|/Script/Engine.CharacterMovementComponent|GetCurrentFloor (Variables|Character|GetCharacterMovement)))
    ;[1 0.09896 0.09896] If is not the case, we want to rotate
    (if (not (> (Utilities|Array|Length (Collision|GetOverlappingActors (Variables|Default|GetLedgeDetector) 0 :!class /Script/Engine.PrimitiveComponent)) 0))
      (CallFunction|RotateCharacter))))