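; King character Blueprint that sets up Enhanced Input for its player and stubs out jump and move actions.
; BeginPlay runs the parent logic, then casts the controller to PlayerController and adds the IC_CorreMlk mapping context.
; IA_Jump and IA_Move only print debug strings when started, with no movement logic in this graph.
; The construction script only calls its parent.
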(event Input|EnhancedActionEvents|EnhancedInputActionIA_Jump
  (params (ActionValue :type Boolean) (ElapsedSeconds :type Float%20%28double-precision%29) (TriggeredSeconds :type Float%20%28double-precision%29) (InputAction :type Input%20Action%20Object%20Reference :default "/Game/Input/Actions/IA_Jump.IA_Jump"))
  ;[0.429 1 0.5083] This is responsible to control the jump actions of this character
  (:Started
    (Development|PrintString "JUMP")))

(event Input|EnhancedActionEvents|EnhancedInputActionIA_Move
  (params (ActionValue :type Float%20%28double-precision%29) (ElapsedSeconds :type Float%20%28double-precision%29) (TriggeredSeconds :type Float%20%28double-precision%29) (InputAction :type Input%20Action%20Object%20Reference :default "/Game/Input/Actions/IA_Move.IA_Move"))
  ;[0.5246 0.3095 1] This is responsible to control the move actions of this character
  (:Started
    (Development|PrintString "MOVE")))

(event EventBeginPlay
  ;[1 0.3083 0.7353] This is needed to call parent begin play
  (|CallParentFunction)
  ;[1 0.1456 0.7864] Setting the controller
  (bind _asplayer_controller (Utilities|Casting|CastToPlayerController (Pawn|GetController)))
  (Input|AddMappingContext (PlayerController|LocalPlayerSubsystems|GetEnhancedInputLocalPlayerSubsystem _asplayer_controller) "/Game/Input/IC_CorreMlk.IC_CorreMlk" 0 "(bIgnoreAllPressedKeysUntilRelease=True,bForceImmediately=False,bNotifyUserSettings=False)"))

(fn ConstructionScript
  (|CallParentFunction))