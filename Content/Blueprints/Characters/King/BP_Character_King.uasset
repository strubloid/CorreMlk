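; BP_Character_King is the player character for side-scrolling platforming, using Enhanced Input to jump and move along world X.
; Each tick it sets controller yaw from X velocity to face left or right.
; Overlapping an enemy while falling defeats it and bounces the King upward; any other enemy contact defeats the King.
; Defeat removes the input mapping, detaches the spring arm in world space, and plays a sound and camera shake.
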(event OnComponentBeginOverlap(CapsuleComponent)
  (params (OverlappedComponent :type Primitive%20Component%20Object%20Reference) (OtherActor :type Actor%20Object%20Reference) (OtherComp :type Primitive%20Component%20Object%20Reference) (OtherBodyIndex :type Integer) (bFromSweep :type Boolean) (SweepResult :type Hit%20Result%20Structure%20%28by%20ref%29))
  ;[0.4429 0.8898 1] This is for noticing when the enemy touches your character
  (bind _asbp_character_enemy (Utilities|Casting|CastToBP_Character_Enemy OtherActor))
  (if (and (AI|Components|NavMovement|IsFalling (Variables|Character|GetCharacterMovement)) (< (.z (Transformation|GetVelocity)) 0.0))
    ;;[0.1535 0.6128 0.1189] Defeat Enemy
    (Default|Defeat _asbp_character_enemy)
    ;;[1 0.957 0.1669] After we kill we are bouncing up a bit
    (Character|LaunchCharacter (Math|Vector|MakeVector 0.0 0.0 (Variables|Default|GetEnemyBounceLunch)) false true)
    (else
      ;;[1 0 0] Dead
      (CallFunction|Defeat))))

(event Input|EnhancedActionEvents|EnhancedInputActionIA_Jump
  (params (ActionValue :type Boolean) (ElapsedSeconds :type Float%20%28double-precision%29) (TriggeredSeconds :type Float%20%28double-precision%29) (InputAction :type Input%20Action%20Object%20Reference :default "/Game/Input/Actions/IA_Jump.IA_Jump"))
  ;[0.429 1 0.5083] This is responsible to control the jump actions of this character
  (:Started
    (Character|Jump))
  (:Completed
    (Character|StopJumping)))

(event Input|EnhancedActionEvents|EnhancedInputActionIA_Move
  (params (ActionValue :type Float%20%28double-precision%29) (ElapsedSeconds :type Float%20%28double-precision%29) (TriggeredSeconds :type Float%20%28double-precision%29) (InputAction :type Input%20Action%20Object%20Reference :default "/Game/Input/Actions/IA_Move.IA_Move"))
  ;[0.5246 0.3095 1] This is responsible to control the move actions of this character
  (Pawn|Input|AddMovementInput "1.000000,0.000000,0.000000" ActionValue false))

(event EventBeginPlay
  ;[1 0.3083 0.7353] This is needed to call parent begin play
  (|CallParentFunction)
  ;[1 0.1456 0.7864] Setting the controller
  (bind _asplayer_controller (Utilities|Casting|CastToPlayerController (Pawn|GetController)))
  (Input|AddMappingContext (PlayerController|LocalPlayerSubsystems|GetEnhancedInputLocalPlayerSubsystem _asplayer_controller) "/Game/Input/IC_CorreMlk.IC_CorreMlk" 0 "(bIgnoreAllPressedKeysUntilRelease=True,bForceImmediately=False,bNotifyUserSettings=False)"))

(event EventTick
  (params (DeltaSeconds :type Float%20%28single-precision%29))
  (|CallParentFunction DeltaSeconds)
  ;[1 1 1] At every frame this function will check if the character will be going to left or right
  (CallFunction|UpdateControllerRotation))

(event EventDefeat
  (|CallParentFunction)
  ;[1 0.05729 0.05729] When you lose, you must lose the hability of move your own character, as you lost the game
  (bind _asplayer_controller (Utilities|Casting|CastToPlayerController (Pawn|GetController)))
  (Input|RemoveMappingContext (PlayerController|LocalPlayerSubsystems|GetEnhancedInputLocalPlayerSubsystem _asplayer_controller) "/Game/Input/IC_CorreMlk.IC_CorreMlk" "(bIgnoreAllPressedKeysUntilRelease=True,bForceImmediately=False,bNotifyUserSettings=False)")
  ;[1 0.19 0.02604] Now we are detaching from the camera, so you are dead and that is it!
  (Transformation|DetachFromComponent (Variables|Default|GetSpringArm) "KeepWorld" "KeepRelative" "KeepRelative" true)
  ;[1 0 0] What death sounds like ;0
  (Audio|PlaySound2D "/Game/Sounds/PlayerDefeated/S_PlayerDefeated_Cue.S_PlayerDefeated_Cue" 1.0 1.0 0.0 0 0)
  ;[0.9014 1 0.4993] This is the run of the came shake
  (Camera|PlayWorldCameraShake "/Game/CameraShake/CS_Defeated.CS_Defeated_C" (Transformation|GetActorLocation) 0.0 (Variables|Default|GetRadiousAfterDeath) 0.0))

(fn ConstructionScript
  (|CallParentFunction))

(fn UpdateControllerRotation
  (bind _returnvalue (Pawn|GetController))
  (bind _returnvalue_2 (Pawn|GetController))
  ;[1 1 1] Getting character moviment and by checking if the value is bigger, lower or equal to 0
  (Math|Float|CompareFloat (.x (Variables|/Script/Engine.MovementComponent|GetVelocity (Variables|Character|GetCharacterMovement))) 0.0
    (:>
      ;[0.4686 0.4316 1] Right: We don't need to do anything as the basic is to move right
      (Utilities|IsValid _returnvalue_2
        (:Is%20Valid
          (Pawn|SetControlRotation _returnvalue_2 (Math|Rotator|MakeRotator 0.0 0.0 0.0)))))
    (:<
      ;[0.8181 1 0.6561] Left: We need to change the position to go left (z 180)
      (Utilities|IsValid _returnvalue
        (:Is%20Valid
          (Pawn|SetControlRotation _returnvalue (Math|Rotator|MakeRotator 0.0 0.0 1.8e+02)))))))